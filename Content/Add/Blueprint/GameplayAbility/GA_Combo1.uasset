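; Gameplay ability for the first hit of the player's melee combo, notifying the player pawn through Blueprint interface messages.
; On activation it commits, then three parallel delays time the input buffer and damage window start, the combo transition and damage window end, and the ability's end.
; Gameplay tags mark when Combo2 is ready and can begin; on end it removes the Ready tag and signals combo end.
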(event Ability|EventActivateAbility
  (bind _returnvalue (Game|Player|GetPlayerPawn 0))
  (Ability|CommitAbility)
  (Class|BPIPlayer|BPIPlayerCombo(Message) (Game|Player|GetPlayerPawn 0) 1)
  (Utilities|FlowControl|Sequence
    (:then_0
      (Utilities|FlowControl|Delay 0.2) ; インプット先行受付
      (Class|ComboGameplayAbility|AddGameplayTags "(GameplayTags=((TagName=\"Ability.Ready.Combo2\")))")
      (Class|BPIPlayer|BPIPlayerComboDamage(Message) _returnvalue 1) ; ダメージ判定開始
    )
    (:then_1
      (Utilities|FlowControl|Delay 0.3) ; コンボ遷移可能
      (Class|ComboGameplayAbility|AddGameplayTags "(GameplayTags=((TagName=\"Ability.Begin.Combo2\")))")
      (Class|BPIPlayer|BPIPlayerComboDamageEnd(Message) _returnvalue) ; ダメージ判定終了
    )
    (:then_2
      (Utilities|FlowControl|Delay 0.6) ; コンボ1終了
      (Ability|EndAbility))))

(event Ability|EventOnEndAbility
  (params (bWasCancelled :type Boolean))
  (Class|ComboGameplayAbility|RemoveGameplayTags "(GameplayTags=((TagName=\"Ability.Ready.Combo2\"),(TagName=\"Ability.Begin.Combo2\")))")
  (Class|BPIPlayer|BPIPlayerComboEnd(Message) (Game|Player|GetPlayerPawn 0) 1))