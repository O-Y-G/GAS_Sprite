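; Gameplay Ability for the third step of the player's combo attack, committed on activation and started once the Ability.Begin.Combo3 tag is added.
; It drives player pawn 0 through Blueprint interface messages for combo start, damage start, damage end and, on ability end, combo end.
; Parallel Sequence delays, timed from the tag, mark early input, combo transition, input close by tag removal, and ability end.
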(event Ability|EventActivateAbility
  (bind _returnvalue (Game|Player|GetPlayerPawn 0))
  (Ability|CommitAbility)
  (Ability|Tasks|WaitGameplayTagAdd "(TagName=\"Ability.Begin.Combo3\")" 0 true
    (:Added
      (Class|BPIPlayer|BPIPlayerCombo(Message) (Game|Player|GetPlayerPawn 0) 3)
      (Utilities|FlowControl|Sequence
        (:then_0
          (Utilities|FlowControl|Delay 0.3) ; 先行入力
          (Class|BPIPlayer|BPIPlayerComboDamage(Message) _returnvalue 3))
        (:then_1
          (Utilities|FlowControl|Delay 0.6) ; コンボ遷移可能
          (Class|BPIPlayer|BPIPlayerComboDamageEnd(Message) _returnvalue))
        (:then_2
          (Utilities|FlowControl|Delay 1.0) ; 入力受付終了
          (Class|ComboGameplayAbility|RemoveGameplayTags "(GameplayTags=((TagName=\"Ability.Begin.Combo3\"),(TagName=\"Ability.Ready.Combo3\")))"))
        (:then_3
          (Utilities|FlowControl|Delay 1.266) ; コンボ3終了
          (Ability|EndAbility))))))

(event Ability|EventOnEndAbility
  (params (bWasCancelled :type Boolean))
  (Class|BPIPlayer|BPIPlayerComboEnd(Message) (Game|Player|GetPlayerPawn 0) 3))