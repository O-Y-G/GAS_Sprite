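; GA_Combo2 is the gameplay ability for the second step of the player's combo attack.
; After commit it waits once for the Begin.Combo2 tag, then notifies player pawn 0 through interface messages that the step has started.
; Parallel timed delays open and close the damage window, add the Ready and Begin tags for Combo3, and end the ability.
; On end it removes Begin.Combo3 and signals the pawn that step 2 is over.
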(event Ability|EventActivateAbility
  (bind _returnvalue (Game|Player|GetPlayerPawn 0))
  (Ability|CommitAbility)
  (Ability|Tasks|WaitGameplayTagAdd "(TagName=\"Ability.Begin.Combo2\")" 0 true
    (:Added
      (Class|BPIPlayer|BPIPlayerCombo(Message) (Game|Player|GetPlayerPawn 0) 2)
      (Utilities|FlowControl|Sequence
        (:then_0
          (Utilities|FlowControl|Delay 0.4)
          (Class|ComboGameplayAbility|AddGameplayTags "(GameplayTags=((TagName=\"Ability.Ready.Combo3\")))")
          (Class|BPIPlayer|BPIPlayerComboDamage(Message) _returnvalue 2))
        (:then_1
          (Utilities|FlowControl|Delay 0.5)
          (Class|ComboGameplayAbility|AddGameplayTags "(GameplayTags=((TagName=\"Ability.Begin.Combo3\")))")
          (Class|BPIPlayer|BPIPlayerComboDamageEnd(Message) _returnvalue))
        (:then_2
          (Utilities|FlowControl|Delay 0.866)
          (Ability|EndAbility))))))

(event Ability|EventOnEndAbility
  (params (bWasCancelled :type Boolean))
  (Class|ComboGameplayAbility|RemoveGameplayTags "(GameplayTags=((TagName=\"Ability.Begin.Combo3\"),(TagName=\"Ability.Ready.Combo3\"),(TagName=\"Ability.Begin.Combo2\"),(TagName=\"Ability.Ready.Combo2\")))")
  (Class|BPIPlayer|BPIPlayerComboEnd(Message) (Game|Player|GetPlayerPawn 0) 2))